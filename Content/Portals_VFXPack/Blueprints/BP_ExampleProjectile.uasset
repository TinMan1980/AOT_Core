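; Example showcase actor for the Portals VFX pack that repeatedly spawns BP_Sphere_Projectiles actors at its own location and attaches them to itself.
; Each spawn randomizes the portal choice, projectile count and delay, with a fixed target radius.
; Spawning fires on BeginPlay and repeats about every six seconds through a Delay on Tick.
; A Movement timeline for offsetting the actor along Y exists but never runs.
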(event `self.ReceiveBeginPlay`
  (`|ExecutionSequence` :!label _label
    (:`then_0`
      (bind _returnvalue (`|SpawnActorFromClass` "/Game/Portals_VFXPack/Blueprints/BP_Sphere_Projectiles.BP_Sphere_Projectiles_C" (`KismetMathLibrary.MakeTransform` (`self.K2_GetActorLocation`)) "Undefined" "OverrideRootScale" null (`KismetMathLibrary.RandomIntegerInRange` 1 8) 3.0 (`KismetMathLibrary.RandomIntegerInRange` 1 10) (`KismetMathLibrary.RandomFloatInRange` 0.1 0.3) 1000.0 null))
      (`self.K2_AttachToActor` _returnvalue self "None" "SnapToTarget" "KeepRelative" "KeepRelative" true))))

(event `self.ReceiveTick`
  (params (DeltaSeconds :type "Float (single-precision)"))
  (`KismetSystemLibrary.Delay` 6.0)
  (goto _label))

(fn `UserConstructionScript`)