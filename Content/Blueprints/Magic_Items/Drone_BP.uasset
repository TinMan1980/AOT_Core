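; Drone actor in the magic items set that exposes movement commands: forward, backward, turn, ascend, descend, face and return.
; Timelines sweep the static mesh forward or back, with the Forawrd flag gating speed boosts and braking, though nothing here sets it true.
; Reverse stops its timeline on each update, while turns and altitude changes are fixed actor steps.
; Facing and the eased return both target the Remote actor's location.
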(event `self.ReceiveBeginPlay`)

(event `/Game/Blueprints/Interfaces/Drone.MoveForward`
  (if (`self.Forawrd`)
    (set `self.DroneSpeed` (+ (`self.DroneSpeed`) 100.0))
    (else
      (bind (_direction _forwardmovementalpha) (`Timeline|ForwardMove` :!label _label)
        (:`Update`
          (`SceneComponent.K2_AddWorldOffset` (`self.StaticMesh`) (`KismetMathLibrary.VLerp` (0.0 0.0 0.0) (* (`self.GetActorForwardVector`) (`self.DroneSpeed`)) _forwardmovementalpha) true false))))))

(event `/Game/Blueprints/Interfaces/Drone.MoveBackward`
  (if (`self.Forawrd`)
    (set `self.Forawrd` false)
    (set `self.DroneSpeed` 500.0)
    (goto _label :!via `Stop`)
    (else
      (bind (_direction _forwardmovementalpha) (`Timeline|Timeline` :!label _label_2)
        (:`Update`
          (`SceneComponent.K2_AddWorldOffset` (`self.StaticMesh`) (`KismetMathLibrary.VLerp` (0.0 0.0 0.0) (* (`self.GetActorForwardVector`) -500.0) _forwardmovementalpha) true false)
          (`self.stop reverse`))))))

(event `stop reverse`
  (goto _label_2 :!via `Stop`))

(event `/Game/Blueprints/Interfaces/Drone.TurnLeft`
  (`self.K2_AddActorLocalRotation` (`KismetMathLibrary.MakeRotator` 0.0 0.0 -15.0)))

(event `/Game/Blueprints/Interfaces/Drone.TurnRight`
  (`self.K2_AddActorLocalRotation` (`KismetMathLibrary.MakeRotator` 0.0 0.0 15.0)))

(event `/Game/Blueprints/Interfaces/Drone.Ascend`
  (`self.K2_AddActorWorldOffset` (0.0 0.0 50.0) true))

(event `/Game/Blueprints/Interfaces/Drone.Descend`
  (`self.K2_AddActorWorldOffset` (0.0 0.0 -50.0) true))

(event `/Game/Blueprints/Interfaces/Drone.FaceCharacter`
  (`self.K2_SetActorRotation` (`KismetMathLibrary.FindLookAtRotation` (`self.K2_GetActorLocation`) (`self.K2_GetActorLocation` (`self.Remote`)))))

(event `/Game/Blueprints/Interfaces/Drone.ReturnToPlayer`
  (bind _returnvalue (`self.K2_GetActorLocation` (`self.Remote`)))
  (`self.K2_SetActorRotation` (`KismetMathLibrary.FindLookAtRotation` (`self.K2_GetActorLocation`) _returnvalue))
  (`KismetSystemLibrary.MoveComponentTo` null _returnvalue (struct) true true 3.0))

(fn `UserConstructionScript`)