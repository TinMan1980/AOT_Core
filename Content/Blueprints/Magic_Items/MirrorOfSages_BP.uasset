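; Mirror of Sages magic item that displays the stats of an AOT_FB_Char's equipped ring while that character stands inside its trigger box.
; Box overlap caches the ring, shows the text components and starts a looping timer that refreshes their values.
; SetStatText builds each label from the component's object name plus the value.
; Leaving the box stops the timer, resets and hides the text, and clears the ring reference.
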(event `self.Box.OnComponentBeginOverlap`
  (params (OverlappedComponent :type "PrimitiveComponent Object Reference") (OtherActor :type "Actor Object Reference") (OtherComp :type "PrimitiveComponent Object Reference") (OtherBodyIndex :type Integer) (bFromSweep :type Boolean) (SweepResult :type "HitResult Structure (by ref)"))
  (bind _asaot_fb_char (cast `/Game/Blueprints/Character/AOT_FB_Char` OtherActor))
  (set `self.Equiped Ring` (`/Game/Blueprints/Character/AOT_FB_Char.Equiped Ring` _asaot_fb_char))
  (`self.Set Text visibility` true
    (:`NewParam2`
      (bind _returnvalue (`KismetSystemLibrary.K2_SetTimerDelegate` (delegate `Update Stat text`) 0.2 true))
      (set `self.Stat Timer` _returnvalue))))

(event `Update Stat text`
  (`self.GetStats` (stale `self.Box.OnComponentBeginOverlap` _asaot_fb_char)))

(event `self.Box.OnComponentEndOverlap`
  (params (OverlappedComponent :type "PrimitiveComponent Object Reference") (OtherActor :type "Actor Object Reference") (OtherComp :type "PrimitiveComponent Object Reference") (OtherBodyIndex :type Integer))
  (cast `/Game/Blueprints/Character/AOT_FB_Char` OtherActor)
  (`KismetSystemLibrary.K2_ClearAndInvalidateTimerHandle` (`self.Stat Timer`))
  (`self.Reset Stat Text`
    (:`NewParam2`
      (`self.Set Text visibility` false
        (:`NewParam2`
          (set `self.Equiped Ring` null))))))

(fn `UserConstructionScript`)