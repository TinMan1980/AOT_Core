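; TravelDoor is a magic-item portal that opens a chosen level, or quits the game, when the VR pawn overlaps its TeleportBox.
; SwitchLeft and SwitchRight step CurrentLevelIndex and show that level's image on the Plane through a dynamic material instance.
; SetHome and SetExit set the Exit flag and swap the picture.
; Only the image lookup clamps the index to two entries; the level-name lookup uses it unclamped.
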(event `self.ReceiveBeginPlay`)

(event `/Game/Blueprints/Interfaces/Gate.switch left`
  (set `self.exit` false)
  (bind _result (`/Engine/EditorBlueprintResources/StandardMacros.DecrementInt` (`self.CurrentLevelIndex`))
    (:`  `
      (`/Engine/EditorBlueprintResources/StandardMacros.IsValid` (`self.dynamicInstance`)
        (:`Is Valid`
          _)
        (:`Is Not Valid`
          (bind _returnvalue (`PrimitiveComponent.CreateDynamicMaterialInstance` (`self.Plane`) 0 "/Game/Materials/Travel_Picture.Travel_Picture" "None"))))
      (`MaterialInstanceDynamic.SetTextureParameterValue` _returnvalue "LevelImage" (`|GetArrayItem` (`self.LevelImages`) (`KismetMathLibrary.Clamp` _result 0 1)))
      (set `self.dynamicInstance` _returnvalue))))

(event `/Game/Blueprints/Interfaces/Gate.switch right`
  (set `self.exit` false)
  (bind _result (`/Engine/EditorBlueprintResources/StandardMacros.IncrementInt` (`self.CurrentLevelIndex`))
    (:`  `
      (`/Engine/EditorBlueprintResources/StandardMacros.IsValid` (`self.dynamicInstance`)
        (:`Is Valid`
          _)
        (:`Is Not Valid`
          (bind _returnvalue (`PrimitiveComponent.CreateDynamicMaterialInstance` (`self.Plane`) 0 "/Game/Materials/Travel_Picture.Travel_Picture" "None"))))
      (`MaterialInstanceDynamic.SetTextureParameterValue` _returnvalue "LevelImage" (`|GetArrayItem` (`self.LevelImages`) (`KismetMathLibrary.Clamp` _result 0 1)))
      (set `self.dynamicInstance` _returnvalue))))

(event `/Game/Blueprints/Interfaces/Gate.set home`
  (set `self.exit` false)
  (`/Engine/EditorBlueprintResources/StandardMacros.IsValid` (`self.dynamicInstance`)
    (:`Is Valid`
      _)
    (:`Is Not Valid`
      (bind _returnvalue (`PrimitiveComponent.CreateDynamicMaterialInstance` (`self.Plane`) 0 "/Game/Materials/Travel_Picture.Travel_Picture" "None"))
      (set `self.dynamicInstance` _returnvalue)))
  (`MaterialInstanceDynamic.SetTextureParameterValue` _returnvalue "LevelImage" (`self.ExitImage`)))

(event `/Game/Blueprints/Interfaces/Gate.set exit`
  (set `self.exit` true)
  (`/Engine/EditorBlueprintResources/StandardMacros.IsValid` (`self.dynamicInstance`)
    (:`Is Valid`
      _)
    (:`Is Not Valid`
      (bind _returnvalue (`PrimitiveComponent.CreateDynamicMaterialInstance` (`self.Plane`) 0 "/Game/Materials/Travel_Picture.Travel_Picture" "None"))
      (set `self.dynamicInstance` _returnvalue)))
  (`MaterialInstanceDynamic.SetTextureParameterValue` _returnvalue "LevelImage" (`self.Choose`)))

(event `self.TeleportBox.OnComponentBeginOverlap`
  (params (OverlappedComponent :type "PrimitiveComponent Object Reference") (OtherActor :type "Actor Object Reference") (OtherComp :type "PrimitiveComponent Object Reference") (OtherBodyIndex :type Integer) (bFromSweep :type Boolean) (SweepResult :type "HitResult Structure (by ref)"))
  (`|ExecutionSequence`
    (:`then_0`
      (cast `/Game/VRTemplate/Blueprints/VRPawn` OtherActor)
      (if (`self.exit`) :!label _label
        (`KismetSystemLibrary.QuitGame` null "Quit")
        (else
          (`GameplayStatics.OpenLevel` (`|GetArrayItem` (`self.LevelNames`) (`self.CurrentLevelIndex`))))))
    (:`then_1`
      (if (== OtherActor "/Game/VRTemplate/Blueprints/VRPawn.VRPawn")
        (goto _label)))))

(fn `UserConstructionScript`)