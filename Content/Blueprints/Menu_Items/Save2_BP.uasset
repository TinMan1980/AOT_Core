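; Grabbable VR menu item that shows one of a set of menu categories on a text render and takes motion-gesture input.
; Grabbing it adds the weapon input context for the holding hand, and the shoot input starts and ends VR gesture recording.
; Twist left or right scrolls the clamped category index.
; Forward and backward twists reach empty category switches, and the "Loaded"/"Saved" feedback is unconnected.
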(event `self.ReceiveBeginPlay`
  (`SceneComponent.K2_AttachToComponent` (`self.StaticMesh`) (`self.DefaultSceneRoot`) "None" "KeepRelative" "KeepRelative" "KeepRelative" true))

(event `self.GrabComponent.OnGrabbed`
  ;[0.03434 0.03434 0.03434] When the Item is grabbed, enable input and add the Weapon Input Mapping Context. Disable and remove when the item is dropped.
  (`self.EnableInput` (`GameplayStatics.GetPlayerController` 0))
  (`EnhancedInputSubsystemInterface.AddMappingContext` (pcsubsystem `EnhancedInputLocalPlayerSubsystem` (`GameplayStatics.GetPlayerController` 0)) (select `bool` (`|EnumEquality` (`/Game/VRTemplate/Blueprints/GrabComponent.GetHeldByHand` (`self.GrabComponent`)) "Right") :`false` "/Game/VRTemplate/Input/IMC_Weapon_Left.IMC_Weapon_Left" :`true` "/Game/VRTemplate/Input/IMC_Weapon_Right.IMC_Weapon_Right" :!type "InputMappingContext Object Reference") 0 (struct)))

(event `self.GrabComponent.OnDropped`
  ;[0.03434 0.03434 0.03434] When the Item is grabbed, enable input and add the Weapon Input Mapping Context. Disable and remove when the item is dropped.
  (`self.DisableInput` (`GameplayStatics.GetPlayerController` 0))
  (`EnhancedInputSubsystemInterface.RemoveMappingContext` (pcsubsystem `EnhancedInputLocalPlayerSubsystem` (`GameplayStatics.GetPlayerController` 0)) (select `bool` (`|EnumEquality` (`/Game/VRTemplate/Blueprints/GrabComponent.GetHeldByHand` (`self.GrabComponent`)) "Right") :`false` "/Game/VRTemplate/Input/IMC_Weapon_Left.IMC_Weapon_Left" :`true` "/Game/VRTemplate/Input/IMC_Weapon_Right.IMC_Weapon_Right" :!type "InputMappingContext Object Reference") (struct)))

(event `EnhancedInput|/Game/VRTemplate/Input/Actions/IA_Shoot_Left`
  (params (ActionValue :type Boolean) (ElapsedSeconds :type "Float (double-precision)") (TriggeredSeconds :type "Float (double-precision)") (InputAction :type "InputAction Object Reference" :default "/Game/VRTemplate/Input/Actions/IA_Shoot_Left.IA_Shoot_Left"))
  (:`Started`
    (`self.Get Hand Held` :!label _label
      (:`then`
        _)
      (:`then2`
        _))
    (`self.Gesture Detect` :!label _label_2))
  (:`Completed`
    (`self.Get Hand Held` :!label _label_3
      (:`then`
        (goto _label_2 :!via `execute2`))
      (:`then2`
        (goto _label_2 :!via `execute2`)))))

(event `EnhancedInput|/Game/VRTemplate/Input/Actions/IA_Shoot_Right`
  (params (ActionValue :type Boolean) (ElapsedSeconds :type "Float (double-precision)") (TriggeredSeconds :type "Float (double-precision)") (InputAction :type "InputAction Object Reference" :default "/Game/VRTemplate/Input/Actions/IA_Shoot_Right.IA_Shoot_Right"))
  (:`Started`
    (goto _label :!via `execute2`))
  (:`Completed`
    (goto _label_3 :!via `execute2`)))

(event `EnhancedInput|/Game/VRTemplate/Input/Actions/IA_Cancel_Left`
  (params (ActionValue :type Boolean) (ElapsedSeconds :type "Float (double-precision)") (TriggeredSeconds :type "Float (double-precision)") (InputAction :type "InputAction Object Reference" :default "/Game/VRTemplate/Input/Actions/IA_Cancel_Left.IA_Cancel_Left"))
  (:`Started`
    (`self.Get Hand Held` :!label _label_4)))

(event `EnhancedInput|/Game/VRTemplate/Input/Actions/IA_Cancel_Right`
  (params (ActionValue :type Boolean) (ElapsedSeconds :type "Float (double-precision)") (TriggeredSeconds :type "Float (double-precision)") (InputAction :type "InputAction Object Reference" :default "/Game/VRTemplate/Input/Actions/IA_Cancel_Right.IA_Cancel_Right"))
  (:`Started`
    (goto _label_4 :!via `execute2`)))

(event `EnhancedInput|/Game/VRTemplate/Input/Actions/IA_Gesture_Left`
  (params (ActionValue :type Boolean) (ElapsedSeconds :type "Float (double-precision)") (TriggeredSeconds :type "Float (double-precision)") (InputAction :type "InputAction Object Reference" :default "/Game/VRTemplate/Input/Actions/IA_Gesture_Left.IA_Gesture_Left"))
  (:`Started`
    (`self.Get Hand Held` :!label _label_5)))

(event `EnhancedInput|/Game/VRTemplate/Input/Actions/IA_Gesture_Right`
  (params (ActionValue :type Boolean) (ElapsedSeconds :type "Float (double-precision)") (TriggeredSeconds :type "Float (double-precision)") (InputAction :type "InputAction Object Reference" :default "/Game/VRTemplate/Input/Actions/IA_Gesture_Right.IA_Gesture_Right"))
  (:`Started`
    (goto _label_5 :!via `execute2`)))

(event `Scroll Next`
  (bind _result (`/Engine/EditorBlueprintResources/StandardMacros.IncrementInt` (`self.CurrentCategoryIndex`))
    (:`  `
      (bind _output_get (set `self.CurrentCategoryIndex` (`KismetMathLibrary.Clamp` _result 0 3)))
      (`TextRenderComponent.K2_SetText` (`self.TextRender`) (`KismetTextLibrary.Conv_StringToText` (`|GetArrayItem` (`self.MenuCategories`) _output_get))))))

(event `Scroll Previous`
  (bind _result (`/Engine/EditorBlueprintResources/StandardMacros.DecrementInt` (`self.CurrentCategoryIndex`))
    (:`  `
      (bind _output_get (set `self.CurrentCategoryIndex` (`KismetMathLibrary.Clamp` _result 0 3)))
      (`TextRenderComponent.K2_SetText` (`self.TextRender`) (`KismetTextLibrary.Conv_StringToText` (`|GetArrayItem` (`self.MenuCategories`) _output_get))))))

(event `Turn Up`
  (switch `string` (`|GetArrayItem` (`self.MenuCategories`) (`self.CurrentCategoryIndex`))))

(event `Turn Down`
  (switch `string` (`|GetArrayItem` (`self.MenuCategories`) (`self.CurrentCategoryIndex`))))

(event `self.VRGesture.OnGestureDetected_Bind`
  (params (GestureType :type Byte) (DetectedGestureName :type String) (DetectedGestureIndex :type Integer) (GestureDataBase :type "GesturesDatabase Object Reference") (OriginalUnscaledGestureSize :type "Vector Structure"))
  (`self.Switch on gesture` DetectedGestureName))

(fn `UserConstructionScript`)