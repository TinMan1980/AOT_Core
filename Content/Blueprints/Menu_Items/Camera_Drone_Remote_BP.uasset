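; Grabbable VR remote that spawns or destroys a single camera drone and exposes movement commands through the drone's interface.
; The Game Instance stores the drone reference so a replacement remote can regain control.
; Hand-checked shoot inputs drive VR gesture recording for detection or saving new gestures.
; Detected gesture names appear on a text render, but the switch mapping them to drone commands is disconnected.
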(event `self.ReceiveBeginPlay`
  (`parent.ReceiveBeginPlay`)
  (bind _astest_game_instance (cast `/Game/Blueprints/TestGameInstance` (`GameplayStatics.GetGameInstance`)))
  (bind _controlleddrone (`/Game/Blueprints/TestGameInstance.ControlledDrone` _astest_game_instance))
  (if (`KismetSystemLibrary.IsValid` _controlleddrone)
    (set `self.ControlledDrone` _controlleddrone)))

(event `EnhancedInput|/Game/VRTemplate/Input/Actions/IA_Shoot_Left`
  (params (ActionValue :type Boolean) (ElapsedSeconds :type "Float (double-precision)") (TriggeredSeconds :type "Float (double-precision)") (InputAction :type "InputAction Object Reference" :default "/Game/VRTemplate/Input/Actions/IA_Shoot_Left.IA_Shoot_Left"))
  ;[0.03434 0.03434 0.03434] Input Actions for both Left and Right. We're validating if the correct hand executed the Input Action event in the case of both hands holding the Item
  (:`Started`
    (`self.Get Hand Held` :!label _label
      (:`then`
        _)
      (:`then2`
        _))
    (`self.Gesture Detect` :!label _label_2))
  (:`Completed`
    (`self.Get Hand Held` :!label _label_3
      (:`then`
        (goto _label_2 :!via `execute2`))
      (:`then2`
        (goto _label_2 :!via `execute2`)))))

(event `EnhancedInput|/Game/VRTemplate/Input/Actions/IA_Shoot_Right`
  (params (ActionValue :type Boolean) (ElapsedSeconds :type "Float (double-precision)") (TriggeredSeconds :type "Float (double-precision)") (InputAction :type "InputAction Object Reference" :default "/Game/VRTemplate/Input/Actions/IA_Shoot_Right.IA_Shoot_Right"))
  ;[0.03434 0.03434 0.03434] Input Actions for both Left and Right. We're validating if the correct hand executed the Input Action event in the case of both hands holding the Item
  (:`Started`
    (goto _label :!via `execute2`))
  (:`Completed`
    (goto _label_3 :!via `execute2`)))

(event `EnhancedInput|/Game/VRTemplate/Input/Actions/IA_Cancel_Left`
  (params (ActionValue :type Boolean) (ElapsedSeconds :type "Float (double-precision)") (TriggeredSeconds :type "Float (double-precision)") (InputAction :type "InputAction Object Reference" :default "/Game/VRTemplate/Input/Actions/IA_Cancel_Left.IA_Cancel_Left"))
  ;[0.03434 0.03434 0.03434] Input Actions for both Left and Right. We're validating if the correct hand executed the Input Action event in the case of both hands holding the Item
)

(event `EnhancedInput|/Game/VRTemplate/Input/Actions/IA_Cancel_Right`
  (params (ActionValue :type Boolean) (ElapsedSeconds :type "Float (double-precision)") (TriggeredSeconds :type "Float (double-precision)") (InputAction :type "InputAction Object Reference" :default "/Game/VRTemplate/Input/Actions/IA_Cancel_Right.IA_Cancel_Right"))
  ;[0.03434 0.03434 0.03434] Input Actions for both Left and Right. We're validating if the correct hand executed the Input Action event in the case of both hands holding the Item
)

(event `EnhancedInput|/Game/VRTemplate/Input/Actions/IA_Gesture_Left`
  (params (ActionValue :type Boolean) (ElapsedSeconds :type "Float (double-precision)") (TriggeredSeconds :type "Float (double-precision)") (InputAction :type "InputAction Object Reference" :default "/Game/VRTemplate/Input/Actions/IA_Gesture_Left.IA_Gesture_Left"))
  ;[0.03434 0.03434 0.03434] Input Actions for both Left and Right. We're validating if the correct hand executed the Input Action event in the case of both hands holding the Item
)

(event `EnhancedInput|/Game/VRTemplate/Input/Actions/IA_Gesture_Right`
  (params (ActionValue :type Boolean) (ElapsedSeconds :type "Float (double-precision)") (TriggeredSeconds :type "Float (double-precision)") (InputAction :type "InputAction Object Reference" :default "/Game/VRTemplate/Input/Actions/IA_Gesture_Right.IA_Gesture_Right"))
  ;[0.03434 0.03434 0.03434] Input Actions for both Left and Right. We're validating if the correct hand executed the Input Action event in the case of both hands holding the Item
)

(event `self.GrabComponent.OnGrabbed`
  (`SceneComponent.SetVisibility` (`self.Plane`) true false))

(event `self.GrabComponent.OnDropped`
  (`SceneComponent.SetVisibility` (`self.Plane`) false false))

(event `self.VRGesture.OnGestureDetected_Bind`
  (params (GestureType :type Byte) (DetectedGestureName :type String) (DetectedGestureIndex :type Integer) (GestureDataBase :type "GesturesDatabase Object Reference") (OriginalUnscaledGestureSize :type "Vector Structure"))
  (`TextRenderComponent.K2_SetText` (`self.TextRender`) (`KismetTextLibrary.Conv_StringToText` DetectedGestureName)))

(event `Deploy`
  ;[1 1 1] This Spawns The Drone and uses the game instance to make sure you can only spawn one and can control the same one you spawned even if the remote is destroyed
  (bind _astest_game_instance (cast `/Game/Blueprints/TestGameInstance` (`GameplayStatics.GetGameInstance`)))
  (if (`/Game/Blueprints/TestGameInstance.DroneSpawn` _astest_game_instance)
    (`self.K2_DestroyActor` (`self.ControlledDrone`))
    (set `/Game/Blueprints/TestGameInstance.DroneSpawn` false _astest_game_instance)
    (else
      (bind _returnvalue (`|SpawnActorFromClass` "/Game/Blueprints/Magic_Items/Drone_BP.Drone_BP_C" (`SceneComponent.K2_GetComponentToWorld` (`self.Sphere`)) "AdjustIfPossibleButAlwaysSpawn" "OverrideRootScale" null null))
      (bind _output_get (set `/Game/Blueprints/TestGameInstance.ControlledDrone` _returnvalue _astest_game_instance))
      (set `/Game/Blueprints/TestGameInstance.DroneSpawn` true _astest_game_instance)
      (bind _output_get_2 (set `self.ControlledDrone` _output_get))
      (set `/Game/Blueprints/Magic_Items/Drone_BP.Remote` self _output_get_2))))

(event `MoveDroneForward`
  ;[1 1 1] These events use the drone blueprint interface to send commands to your drone
  (`/Game/Blueprints/Magic_Items/Drone_BP.MoveForward` (`self.ControlledDrone`)))

(event `Move Drone Backward`
  ;[1 1 1] These events use the drone blueprint interface to send commands to your drone
  (`/Game/Blueprints/Magic_Items/Drone_BP.MoveBackward` (`self.ControlledDrone`)))

(event `Turn Drone Left`
  ;[1 1 1] These events use the drone blueprint interface to send commands to your drone
  (`/Game/Blueprints/Magic_Items/Drone_BP.TurnLeft` (`self.ControlledDrone`)))

(event `Turn Drone Right`
  ;[1 1 1] These events use the drone blueprint interface to send commands to your drone
  (`/Game/Blueprints/Magic_Items/Drone_BP.TurnRight` (`self.ControlledDrone`)))

(event `Go up`
  ;[1 1 1] These events use the drone blueprint interface to send commands to your drone
  (`/Game/Blueprints/Magic_Items/Drone_BP.Ascend` (`self.ControlledDrone`)))

(event `go down`
  ;[1 1 1] These events use the drone blueprint interface to send commands to your drone
  (`/Game/Blueprints/Magic_Items/Drone_BP.Descend` (`self.ControlledDrone`)))

(event `Return Drone to player`
  ;[1 1 1] These events use the drone blueprint interface to send commands to your drone
  (`/Game/Blueprints/Magic_Items/Drone_BP.ReturnToPlayer` (`self.ControlledDrone`)))

(event `Look at Player`
  ;[1 1 1] These events use the drone blueprint interface to send commands to your drone
  (`/Game/Blueprints/Magic_Items/Drone_BP.FaceCharacter` (`self.ControlledDrone`)))

(fn `UserConstructionScript`
  (`parent.UserConstructionScript`))