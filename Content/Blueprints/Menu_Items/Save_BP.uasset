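; Save_BP is a grabbable VR item Blueprint among the menu items, apparently a scaffold for a save item, with no save logic in these graphs.
; Left and right Shoot, Cancel and Gesture input events check that GrabComponent is held by the matching hand, so only that hand's input counts.
; Every branch ends empty, and BeginPlay, overlap and Tick are disabled stubs.
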(event `EnhancedInput|/Game/VRTemplate/Input/Actions/IA_Shoot_Left`
  (params (ActionValue :type Boolean) (ElapsedSeconds :type "Float (double-precision)") (TriggeredSeconds :type "Float (double-precision)") (InputAction :type "InputAction Object Reference" :default "/Game/VRTemplate/Input/Actions/IA_Shoot_Left.IA_Shoot_Left"))
  ;[0.03434 0.03434 0.03434] Input Actions for both Left and Right. We're validating if the correct hand executed the Input Action event in the case of both hands holding the Item
  (:`Started`
    (if (`|EnumEquality` (`/Game/VRTemplate/Blueprints/GrabComponent.GetHeldByHand` (`self.GrabComponent`)) "Left")
      _)))

(event `EnhancedInput|/Game/VRTemplate/Input/Actions/IA_Shoot_Right`
  (params (ActionValue :type Boolean) (ElapsedSeconds :type "Float (double-precision)") (TriggeredSeconds :type "Float (double-precision)") (InputAction :type "InputAction Object Reference" :default "/Game/VRTemplate/Input/Actions/IA_Shoot_Right.IA_Shoot_Right"))
  ;[0.03434 0.03434 0.03434] Input Actions for both Left and Right. We're validating if the correct hand executed the Input Action event in the case of both hands holding the Item
  (:`Started`
    (if (`|EnumEquality` (`/Game/VRTemplate/Blueprints/GrabComponent.GetHeldByHand` (`self.GrabComponent`)) "Right")
      _)))

(event `EnhancedInput|/Game/VRTemplate/Input/Actions/IA_Cancel_Left`
  (params (ActionValue :type Boolean) (ElapsedSeconds :type "Float (double-precision)") (TriggeredSeconds :type "Float (double-precision)") (InputAction :type "InputAction Object Reference" :default "/Game/VRTemplate/Input/Actions/IA_Cancel_Left.IA_Cancel_Left"))
  ;[0.03434 0.03434 0.03434] Input Actions for both Left and Right. We're validating if the correct hand executed the Input Action event in the case of both hands holding the Item
  (:`Started`
    (if (`|EnumEquality` (`/Game/VRTemplate/Blueprints/GrabComponent.GetHeldByHand` (`self.GrabComponent`)) "Left")
      _)))

(event `EnhancedInput|/Game/VRTemplate/Input/Actions/IA_Cancel_Right`
  (params (ActionValue :type Boolean) (ElapsedSeconds :type "Float (double-precision)") (TriggeredSeconds :type "Float (double-precision)") (InputAction :type "InputAction Object Reference" :default "/Game/VRTemplate/Input/Actions/IA_Cancel_Right.IA_Cancel_Right"))
  ;[0.03434 0.03434 0.03434] Input Actions for both Left and Right. We're validating if the correct hand executed the Input Action event in the case of both hands holding the Item
  (:`Started`
    (if (`|EnumEquality` (`/Game/VRTemplate/Blueprints/GrabComponent.GetHeldByHand` (`self.GrabComponent`)) "Right")
      _)))

(event `EnhancedInput|/Game/VRTemplate/Input/Actions/IA_Gesture_Left`
  (params (ActionValue :type Boolean) (ElapsedSeconds :type "Float (double-precision)") (TriggeredSeconds :type "Float (double-precision)") (InputAction :type "InputAction Object Reference" :default "/Game/VRTemplate/Input/Actions/IA_Gesture_Left.IA_Gesture_Left"))
  ;[0.03434 0.03434 0.03434] Input Actions for both Left and Right. We're validating if the correct hand executed the Input Action event in the case of both hands holding the Item
  (:`Started`
    (if (`|EnumEquality` (`/Game/VRTemplate/Blueprints/GrabComponent.GetHeldByHand` (`self.GrabComponent`)) "Left")
      _)))

(event `EnhancedInput|/Game/VRTemplate/Input/Actions/IA_Gesture_Right`
  (params (ActionValue :type Boolean) (ElapsedSeconds :type "Float (double-precision)") (TriggeredSeconds :type "Float (double-precision)") (InputAction :type "InputAction Object Reference" :default "/Game/VRTemplate/Input/Actions/IA_Gesture_Right.IA_Gesture_Right"))
  ;[0.03434 0.03434 0.03434] Input Actions for both Left and Right. We're validating if the correct hand executed the Input Action event in the case of both hands holding the Item
  (:`Started`
    (if (`|EnumEquality` (`/Game/VRTemplate/Blueprints/GrabComponent.GetHeldByHand` (`self.GrabComponent`)) "Right")
      _)))

(fn `UserConstructionScript`
  (`parent.UserConstructionScript`))