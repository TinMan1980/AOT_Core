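; Grabbable VR travel item that summons and controls a TravelDoor_BP through hand gestures.
; While held, it adds the hand's weapon input context, whose shoot action starts and ends VRGesture recording.
; The Door gesture toggles a door spawned by downward trace at a world-X offset, while twists scroll it or set Home/Exit.
; A looping timer snaps the root to the mesh, and destroying the item destroys its door.
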(event `self.ReceiveBeginPlay`
  (`KismetSystemLibrary.K2_SetTimerDelegate` (delegate `UpdateScene Location`) 0.08 true)
  (add `self.OnDestroyed` (delegate `OnDestroyed_Event`)))

(event `UpdateScene Location`
  (`SceneComponent.K2_SetWorldTransform` (`self.DefaultSceneRoot`) (`SceneComponent.K2_GetComponentToWorld` (`self.StaticMesh`)) false false))

(event `OnDestroyed_Event` :!signature `self.OnDestroyed`
  (params (DestroyedActor :type "Actor Object Reference"))
  (`self.K2_DestroyActor` (`self.Summoned_Door`)))

(event `self.GrabComponent.OnGrabbed`
  ;[0.03434 0.03434 0.03434] When the Item is grabbed, enable input and add the Weapon Input Mapping Context. Disable and remove when the item is dropped.
  (`self.EnableInput` (`GameplayStatics.GetPlayerController` 0))
  (`EnhancedInputSubsystemInterface.AddMappingContext` (pcsubsystem `EnhancedInputLocalPlayerSubsystem` (`GameplayStatics.GetPlayerController` 0)) (select `bool` (`|EnumEquality` (`/Game/VRTemplate/Blueprints/GrabComponent.GetHeldByHand` (`self.GrabComponent`)) "Right") :`false` "/Game/VRTemplate/Input/IMC_Weapon_Left.IMC_Weapon_Left" :`true` "/Game/VRTemplate/Input/IMC_Weapon_Right.IMC_Weapon_Right" :!type "InputMappingContext Object Reference") 0 (struct)))

(event `self.GrabComponent.OnDropped`
  ;[0.03434 0.03434 0.03434] When the Item is grabbed, enable input and add the Weapon Input Mapping Context. Disable and remove when the item is dropped.
  (`self.DisableInput` (`GameplayStatics.GetPlayerController` 0))
  (`EnhancedInputSubsystemInterface.RemoveMappingContext` (pcsubsystem `EnhancedInputLocalPlayerSubsystem` (`GameplayStatics.GetPlayerController` 0)) (select `bool` (`|EnumEquality` (`/Game/VRTemplate/Blueprints/GrabComponent.GetHeldByHand` (`self.GrabComponent`)) "Right") :`false` "/Game/VRTemplate/Input/IMC_Weapon_Left.IMC_Weapon_Left" :`true` "/Game/VRTemplate/Input/IMC_Weapon_Right.IMC_Weapon_Right" :!type "InputMappingContext Object Reference") (struct)))

(event `EnhancedInput|/Game/VRTemplate/Input/Actions/IA_Shoot_Left`
  (params (ActionValue :type Boolean) (ElapsedSeconds :type "Float (double-precision)") (TriggeredSeconds :type "Float (double-precision)") (InputAction :type "InputAction Object Reference" :default "/Game/VRTemplate/Input/Actions/IA_Shoot_Left.IA_Shoot_Left"))
  (:`Started`
    (`self.Get Hand Held` :!label _label
      (:`then`
        _)
      (:`then2`
        _))
    (`self.Gesture Detect` :!label _label_2))
  (:`Completed`
    (`self.Get Hand Held` :!label _label_3
      (:`then`
        (goto _label_2 :!via `execute2`))
      (:`then2`
        (goto _label_2 :!via `execute2`)))))

(event `EnhancedInput|/Game/VRTemplate/Input/Actions/IA_Shoot_Right`
  (params (ActionValue :type Boolean) (ElapsedSeconds :type "Float (double-precision)") (TriggeredSeconds :type "Float (double-precision)") (InputAction :type "InputAction Object Reference" :default "/Game/VRTemplate/Input/Actions/IA_Shoot_Right.IA_Shoot_Right"))
  (:`Started`
    (goto _label :!via `execute2`))
  (:`Completed`
    (goto _label_3 :!via `execute2`)))

(event `EnhancedInput|/Game/VRTemplate/Input/Actions/IA_Cancel_Left`
  (params (ActionValue :type Boolean) (ElapsedSeconds :type "Float (double-precision)") (TriggeredSeconds :type "Float (double-precision)") (InputAction :type "InputAction Object Reference" :default "/Game/VRTemplate/Input/Actions/IA_Cancel_Left.IA_Cancel_Left")))

(event `EnhancedInput|/Game/VRTemplate/Input/Actions/IA_Cancel_Right`
  (params (ActionValue :type Boolean) (ElapsedSeconds :type "Float (double-precision)") (TriggeredSeconds :type "Float (double-precision)") (InputAction :type "InputAction Object Reference" :default "/Game/VRTemplate/Input/Actions/IA_Cancel_Right.IA_Cancel_Right")))

(event `EnhancedInput|/Game/VRTemplate/Input/Actions/IA_Gesture_Left`
  (params (ActionValue :type Boolean) (ElapsedSeconds :type "Float (double-precision)") (TriggeredSeconds :type "Float (double-precision)") (InputAction :type "InputAction Object Reference" :default "/Game/VRTemplate/Input/Actions/IA_Gesture_Left.IA_Gesture_Left")))

(event `EnhancedInput|/Game/VRTemplate/Input/Actions/IA_Gesture_Right`
  (params (ActionValue :type Boolean) (ElapsedSeconds :type "Float (double-precision)") (TriggeredSeconds :type "Float (double-precision)") (InputAction :type "InputAction Object Reference" :default "/Game/VRTemplate/Input/Actions/IA_Gesture_Right.IA_Gesture_Right")))

(event `self.VRGesture.OnGestureDetected_Bind`
  (params (GestureType :type Byte) (DetectedGestureName :type String) (DetectedGestureIndex :type Integer) (GestureDataBase :type "GesturesDatabase Object Reference") (OriginalUnscaledGestureSize :type "Vector Structure"))
  (`self.Switch on gesture` DetectedGestureName))

(event `Scroll Next`
  (`/Game/Blueprints/Interfaces/Gate.switch left` (`self.Summoned_Door`)))

(event `Scroll Previous`
  (`/Game/Blueprints/Interfaces/Gate.switch right` (`self.Summoned_Door`)))

(event `Set Door to Exit`
  (`/Game/Blueprints/Interfaces/Gate.set exit` (`self.Summoned_Door`)))

(event `Set door to Home`
  (`/Game/Blueprints/Interfaces/Gate.set home` (`self.Summoned_Door`)))

(event `Summon Door`
  (bind _returnvalue (`SceneComponent.K2_GetComponentLocation` (`self.StaticMesh`)))
  (if (`self.Door`)
    (`self.K2_DestroyActor` (stale _returnvalue_4))
    (set `self.Door` false)
    (else
      (bind (_outhit _returnvalue_2) (`KismetSystemLibrary.LineTraceSingle` (+ _returnvalue (250.0 0.0 1000.0)) (+ _returnvalue (250.0 0.0 -5000.0)) "TraceTypeQuery1"))
      (if _returnvalue_2
        (bind _returnvalue_3 (+ (`.Location` (`GameplayStatics.BreakHitResult` _outhit)) (0.0 0.0 5.0)))
        (bind (_returnvalue_roll _returnvalue_pitch _returnvalue_yaw) (`KismetMathLibrary.BreakRotator` (`KismetMathLibrary.FindLookAtRotation` _returnvalue_3 (`SceneComponent.K2_GetComponentLocation` (`self.StaticMesh`)))))
        (bind _returnvalue_4 (`|SpawnActorFromClass` "/Game/Blueprints/Magic_Items/TravelDoor_BP.TravelDoor_BP_C" (`KismetMathLibrary.MakeTransform` _returnvalue_3 (`KismetMathLibrary.MakeRotator` _returnvalue_roll 0.0 _returnvalue_yaw)) "Undefined" "OverrideRootScale" null null))
        (set `self.Door` true)
        (set `self.Summoned_Door` _returnvalue_4)))))

(fn `UserConstructionScript`)