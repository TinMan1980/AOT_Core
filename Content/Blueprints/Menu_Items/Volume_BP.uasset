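; Volume_BP is a held VR menu item, a work-in-progress gesture-driven control for Music, Background, Effects and Dialogue volume categories.
; Shoot input from the holding hand starts and ends VRGesture capture, with a Recording flag choosing gesture saving over detection.
; Detected gesture names display on a TextRender, but the twist-to-action switch is unconnected.
; Scroll events change category, while TurnUp and TurnDown only flash text, without adjusting volume.
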(event `EnhancedInput|/Game/VRTemplate/Input/Actions/IA_Shoot_Left`
  (params (ActionValue :type Boolean) (ElapsedSeconds :type "Float (double-precision)") (TriggeredSeconds :type "Float (double-precision)") (InputAction :type "InputAction Object Reference" :default "/Game/VRTemplate/Input/Actions/IA_Shoot_Left.IA_Shoot_Left"))
  ;[0.03434 0.03434 0.03434] Input Actions for both Left and Right. We're validating if the correct hand executed the Input Action event in the case of both hands holding the Item
  (:`Started`
    (`self.Get Hand Held` :!label _label
      (:`then`
        _)
      (:`then2`
        _))
    (`self.Gesture Detect` :!label _label_2))
  (:`Completed`
    (`self.Get Hand Held` :!label _label_3
      (:`then`
        (goto _label_2 :!via `execute2`))
      (:`then2`
        (goto _label_2 :!via `execute2`)))))

(event `EnhancedInput|/Game/VRTemplate/Input/Actions/IA_Shoot_Right`
  (params (ActionValue :type Boolean) (ElapsedSeconds :type "Float (double-precision)") (TriggeredSeconds :type "Float (double-precision)") (InputAction :type "InputAction Object Reference" :default "/Game/VRTemplate/Input/Actions/IA_Shoot_Right.IA_Shoot_Right"))
  ;[0.03434 0.03434 0.03434] Input Actions for both Left and Right. We're validating if the correct hand executed the Input Action event in the case of both hands holding the Item
  (:`Started`
    (goto _label :!via `execute2`))
  (:`Completed`
    (goto _label_3 :!via `execute2`)))

(event `EnhancedInput|/Game/VRTemplate/Input/Actions/IA_Cancel_Left`
  (params (ActionValue :type Boolean) (ElapsedSeconds :type "Float (double-precision)") (TriggeredSeconds :type "Float (double-precision)") (InputAction :type "InputAction Object Reference" :default "/Game/VRTemplate/Input/Actions/IA_Cancel_Left.IA_Cancel_Left"))
  ;[0.03434 0.03434 0.03434] Input Actions for both Left and Right. We're validating if the correct hand executed the Input Action event in the case of both hands holding the Item
)

(event `EnhancedInput|/Game/VRTemplate/Input/Actions/IA_Cancel_Right`
  (params (ActionValue :type Boolean) (ElapsedSeconds :type "Float (double-precision)") (TriggeredSeconds :type "Float (double-precision)") (InputAction :type "InputAction Object Reference" :default "/Game/VRTemplate/Input/Actions/IA_Cancel_Right.IA_Cancel_Right"))
  ;[0.03434 0.03434 0.03434] Input Actions for both Left and Right. We're validating if the correct hand executed the Input Action event in the case of both hands holding the Item
)

(event `EnhancedInput|/Game/VRTemplate/Input/Actions/IA_Gesture_Left`
  (params (ActionValue :type Boolean) (ElapsedSeconds :type "Float (double-precision)") (TriggeredSeconds :type "Float (double-precision)") (InputAction :type "InputAction Object Reference" :default "/Game/VRTemplate/Input/Actions/IA_Gesture_Left.IA_Gesture_Left"))
  ;[0.03434 0.03434 0.03434] Input Actions for both Left and Right. We're validating if the correct hand executed the Input Action event in the case of both hands holding the Item
)

(event `EnhancedInput|/Game/VRTemplate/Input/Actions/IA_Gesture_Right`
  (params (ActionValue :type Boolean) (ElapsedSeconds :type "Float (double-precision)") (TriggeredSeconds :type "Float (double-precision)") (InputAction :type "InputAction Object Reference" :default "/Game/VRTemplate/Input/Actions/IA_Gesture_Right.IA_Gesture_Right"))
  ;[0.03434 0.03434 0.03434] Input Actions for both Left and Right. We're validating if the correct hand executed the Input Action event in the case of both hands holding the Item
)

(event `Scroll Next`
  (bind _result (`/Engine/EditorBlueprintResources/StandardMacros.IncrementInt` (`self.CurrentCategoryIndex`))
    (:`  `
      (bind _output_get (set `self.CurrentCategoryIndex` (`KismetMathLibrary.Clamp` _result 0 3)))
      (`TextRenderComponent.K2_SetText` (`self.TextRender`) (`KismetTextLibrary.Conv_StringToText` (`|GetArrayItem` (`self.MenuCategories`) _output_get))))))

(event `Scroll Previous`
  (bind _result (`/Engine/EditorBlueprintResources/StandardMacros.DecrementInt` (`self.CurrentCategoryIndex`))
    (:`  `
      (bind _output_get (set `self.CurrentCategoryIndex` (`KismetMathLibrary.Clamp` _result 0 3)))
      (`TextRenderComponent.K2_SetText` (`self.TextRender`) (`KismetTextLibrary.Conv_StringToText` (`|GetArrayItem` (`self.MenuCategories`) _output_get))))))

(event `Turn Up`
  (bind _output (`|GetArrayItem` (`self.MenuCategories`) (`self.CurrentCategoryIndex`)))
  (switch `string` _output
    (:`Music`
      _)
    (:`Background`
      _)
    (:`Effects`
      _)
    (:`Dialogue`
      _))
  (`TextRenderComponent.K2_SetText` (`self.TextRender`) (`KismetTextLibrary.Conv_StringToText` (`KismetStringLibrary.Concat_StrStr` _output "  " "Up")))
  (`KismetSystemLibrary.Delay` 0.5)
  (`TextRenderComponent.K2_SetText` (`self.TextRender`) (`KismetTextLibrary.Conv_StringToText` (`|GetArrayItem` (`self.MenuCategories`) (`self.CurrentCategoryIndex`)))))

(event `Turn Down`
  (bind _output (`|GetArrayItem` (`self.MenuCategories`) (`self.CurrentCategoryIndex`)))
  (switch `string` _output
    (:`Music`
      _)
    (:`Background`
      _)
    (:`Effects`
      _)
    (:`Dialogue`
      _))
  (`TextRenderComponent.K2_SetText` (`self.TextRender`) (`KismetTextLibrary.Conv_StringToText` (`KismetStringLibrary.Concat_StrStr` _output "  " "Down")))
  (`KismetSystemLibrary.Delay` 0.5)
  (`TextRenderComponent.K2_SetText` (`self.TextRender`) (`KismetTextLibrary.Conv_StringToText` (`|GetArrayItem` (`self.MenuCategories`) (`self.CurrentCategoryIndex`)))))

(event `self.VRGesture.OnGestureDetected_Bind`
  (params (GestureType :type Byte) (DetectedGestureName :type String) (DetectedGestureIndex :type Integer) (GestureDataBase :type "GesturesDatabase Object Reference") (OriginalUnscaledGestureSize :type "Vector Structure"))
  ;[1 1 1] Here is where the gestures do their switching
  (`TextRenderComponent.K2_SetText` (`self.TextRender`) (`KismetTextLibrary.Conv_StringToText` DetectedGestureName)))

(fn `UserConstructionScript`
  (`parent.UserConstructionScript`))