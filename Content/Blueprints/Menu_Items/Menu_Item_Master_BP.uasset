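; Grabbable VR master menu item that records or recognizes motion gestures while held, using a VRGesture component.
; Grabbing adds the left- or right-hand weapon input mapping context, and hand checks filter each input.
; Shoot press and release bound the gesture recording, which either runs detection or saves a named gesture, depending on a Recording flag.
; Detected names briefly show on a TextRender; twist cases and cancel inputs are empty hooks.
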(event `self.GrabComponent.OnGrabbed`
  ;[0.03434 0.03434 0.03434] When the Item is grabbed, enable input and add the Weapon Input Mapping Context. Disable and remove when the item is dropped.
  (`self.EnableInput` (`GameplayStatics.GetPlayerController` 0))
  (`EnhancedInputSubsystemInterface.AddMappingContext` (pcsubsystem `EnhancedInputLocalPlayerSubsystem` (`GameplayStatics.GetPlayerController` 0)) (select `bool` (`|EnumEquality` (`/Game/VRTemplate/Blueprints/GrabComponent.GetHeldByHand` (`self.GrabComponent`)) "Right") :`false` "/Game/VRTemplate/Input/IMC_Weapon_Left.IMC_Weapon_Left" :`true` "/Game/VRTemplate/Input/IMC_Weapon_Right.IMC_Weapon_Right" :!type "InputMappingContext Object Reference") 0 (struct)))

(event `self.GrabComponent.OnDropped`
  ;[0.03434 0.03434 0.03434] When the Item is grabbed, enable input and add the Weapon Input Mapping Context. Disable and remove when the item is dropped.
  (`self.DisableInput` (`GameplayStatics.GetPlayerController` 0))
  (`EnhancedInputSubsystemInterface.RemoveMappingContext` (pcsubsystem `EnhancedInputLocalPlayerSubsystem` (`GameplayStatics.GetPlayerController` 0)) (select `bool` (`|EnumEquality` (`/Game/VRTemplate/Blueprints/GrabComponent.GetHeldByHand` (`self.GrabComponent`)) "Right") :`false` "/Game/VRTemplate/Input/IMC_Weapon_Left.IMC_Weapon_Left" :`true` "/Game/VRTemplate/Input/IMC_Weapon_Right.IMC_Weapon_Right" :!type "InputMappingContext Object Reference") (struct)))

(event `EnhancedInput|/Game/VRTemplate/Input/Actions/IA_Shoot_Left`
  (params (ActionValue :type Boolean) (ElapsedSeconds :type "Float (double-precision)") (TriggeredSeconds :type "Float (double-precision)") (InputAction :type "InputAction Object Reference" :default "/Game/VRTemplate/Input/Actions/IA_Shoot_Left.IA_Shoot_Left"))
  ;[0.03434 0.03434 0.03434] Input Actions for both Left and Right. We're validating if the correct hand executed the Input Action event in the case of both hands holding the Item
  (:`Started`
    (`self.Get Hand Held` :!label _label
      (:`then`
        _)
      (:`then2`
        _))
    (`self.Gesture Detect` :!label _label_2))
  (:`Completed`
    (`self.Get Hand Held` :!label _label_3
      (:`then`
        (goto _label_2 :!via `execute2`))
      (:`then2`
        (goto _label_2 :!via `execute2`)))))

(event `EnhancedInput|/Game/VRTemplate/Input/Actions/IA_Shoot_Right`
  (params (ActionValue :type Boolean) (ElapsedSeconds :type "Float (double-precision)") (TriggeredSeconds :type "Float (double-precision)") (InputAction :type "InputAction Object Reference" :default "/Game/VRTemplate/Input/Actions/IA_Shoot_Right.IA_Shoot_Right"))
  ;[0.03434 0.03434 0.03434] Input Actions for both Left and Right. We're validating if the correct hand executed the Input Action event in the case of both hands holding the Item
  (:`Started`
    (goto _label :!via `execute2`))
  (:`Completed`
    (goto _label_3 :!via `execute2`)))

(event `EnhancedInput|/Game/VRTemplate/Input/Actions/IA_Cancel_Left`
  (params (ActionValue :type Boolean) (ElapsedSeconds :type "Float (double-precision)") (TriggeredSeconds :type "Float (double-precision)") (InputAction :type "InputAction Object Reference" :default "/Game/VRTemplate/Input/Actions/IA_Cancel_Left.IA_Cancel_Left"))
  ;[0.03434 0.03434 0.03434] Input Actions for both Left and Right. We're validating if the correct hand executed the Input Action event in the case of both hands holding the Item
  (:`Started`
    (`self.Get Hand Held` :!label _label_4))
  (:`Completed`
    (`self.Get Hand Held` :!label _label_5)))

(event `EnhancedInput|/Game/VRTemplate/Input/Actions/IA_Cancel_Right`
  (params (ActionValue :type Boolean) (ElapsedSeconds :type "Float (double-precision)") (TriggeredSeconds :type "Float (double-precision)") (InputAction :type "InputAction Object Reference" :default "/Game/VRTemplate/Input/Actions/IA_Cancel_Right.IA_Cancel_Right"))
  ;[0.03434 0.03434 0.03434] Input Actions for both Left and Right. We're validating if the correct hand executed the Input Action event in the case of both hands holding the Item
  (:`Started`
    (goto _label_4 :!via `execute2`))
  (:`Completed`
    (goto _label_5 :!via `execute2`)))

(event `self.VRGesture.OnGestureDetected_Bind`
  (params (GestureType :type Byte) (DetectedGestureName :type String) (DetectedGestureIndex :type Integer) (GestureDataBase :type "GesturesDatabase Object Reference") (OriginalUnscaledGestureSize :type "Vector Structure"))
  ;[1 1 1] This is where the magic happens
  (`self.Switch on gesture` DetectedGestureName))

(fn `UserConstructionScript`)