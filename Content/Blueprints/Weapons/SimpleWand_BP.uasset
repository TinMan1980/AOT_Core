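; Grabbable VR wand that casts spells through GestureTrackerVR gestures, enabling hand-specific Enhanced Input contexts while held.
; Gesture inputs record, save or recognize gestures, with recognized IDs spawning colored fireballs.
; Shooting matches the current spell info against SpellInfoMap and spawns a Project_Spell_Master_BP by form, or an example projectile.
; Element-and-form spell building by gesture and the misfire check exist but are disconnected from live events.
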(event `self.ReceiveBeginPlay`
  (`KismetSystemLibrary.K2_SetTimerDelegate` (delegate `UpdateScene Location`) 0.08 true)
  ;[0.2157 0.4549 1] GestureTrackerVR Start Setup
  (`SceneComponent.K2_AttachToComponent` (`self.GestureTracker`) (`self.Sphere`) "None" "KeepRelative" "KeepRelative" "KeepRelative" false))

(event `UpdateScene Location`
  (bind (_returnvalue_location _returnvalue_rotation) (`KismetMathLibrary.BreakTransform` (`SceneComponent.K2_GetComponentToWorld` (`self.StaticMesh`))))
  (`SceneComponent.K2_SetWorldTransform` (`self.Scene`) (`KismetMathLibrary.MakeTransform` _returnvalue_location _returnvalue_rotation) false false))

(event `self.GrabComponent.OnGrabbed`
  ;[0.03434 0.03434 0.03434] When the Item is grabbed, enable input and add the Weapon Input Mapping Context. Disable and remove when the item is dropped.
  (`self.EnableInput` (`GameplayStatics.GetPlayerController` 0))
  (`EnhancedInputSubsystemInterface.AddMappingContext` (pcsubsystem `EnhancedInputLocalPlayerSubsystem` (`GameplayStatics.GetPlayerController` 0)) (select `bool` (`|EnumEquality` (`/Game/VRTemplate/Blueprints/GrabComponent.GetHeldByHand` (`self.GrabComponent`)) "Right") :`false` "/Game/VRTemplate/Input/IMC_Weapon_Left.IMC_Weapon_Left" :`true` "/Game/VRTemplate/Input/IMC_Weapon_Right.IMC_Weapon_Right" :!type "InputMappingContext Object Reference") 0 (struct))
  (set `self.Player` null))

(event `self.GrabComponent.OnDropped`
  ;[0.03434 0.03434 0.03434] When the Item is grabbed, enable input and add the Weapon Input Mapping Context. Disable and remove when the item is dropped.
  (`self.DisableInput` (`GameplayStatics.GetPlayerController` 0))
  (`EnhancedInputSubsystemInterface.RemoveMappingContext` (pcsubsystem `EnhancedInputLocalPlayerSubsystem` (`GameplayStatics.GetPlayerController` 0)) (select `bool` (`|EnumEquality` (`/Game/VRTemplate/Blueprints/GrabComponent.GetHeldByHand` (`self.GrabComponent`)) "Right") :`false` "/Game/VRTemplate/Input/IMC_Weapon_Left.IMC_Weapon_Left" :`true` "/Game/VRTemplate/Input/IMC_Weapon_Right.IMC_Weapon_Right" :!type "InputMappingContext Object Reference") (struct)))

(event `ContinuousGestureRecognized_Event_0`
  (params (id :type Integer) (name :type String) (recognitionDuration :type "Float (single-precision)") (lengthRatio :type "Float (single-precision)"))
  ;[0.2157 0.4549 1] GestureTrackerVR "Add Gesture Tracker" usage example
  ; If you want you dynamically add your Gesture Tracker it should look something like this.
)

(event `GestureRecognized_Event_0`
  (params (id :type Integer) (name :type String) (recognitionDuration :type "Float (single-precision)") (lengthRatio :type "Float (single-precision)"))
  ;[0.2157 0.4549 1] GestureTrackerVR "Add Gesture Tracker" usage example
  ; If you want you dynamically add your Gesture Tracker it should look something like this.
)

(event `EnhancedInput|/Game/VRTemplate/Input/Actions/IA_Gesture_Left`
  (params (ActionValue :type Boolean) (ElapsedSeconds :type "Float (double-precision)") (TriggeredSeconds :type "Float (double-precision)") (InputAction :type "InputAction Object Reference" :default "/Game/VRTemplate/Input/Actions/IA_Gesture_Left.IA_Gesture_Left"))
  (bind _gesturetracker (`self.GestureTracker`))
  ;[0.2157 0.4549 1] GestureTrackerVR Functions Setup
  (:`Triggered`
    (`self.Get Hand Held` :!label _label
      (:`then`
        _)
      (:`then2`
        _))
    (`GestureTracker.StartRecording` _gesturetracker false))
  (:`Completed`
    (`self.Get Hand Held` :!label _label_2
      (:`then`
        _)
      (:`then2`
        _))
    (`GestureTracker.FinishRecording` _gesturetracker -1 "")))

(event `self.GestureTracker.ContinuousGestureRecognized`
  (params (id :type Integer) (name :type String) (recognitionDuration :type "Float (single-precision)") (lengthRatio :type "Float (single-precision)"))
  ;[0.2157 0.4549 1] GestureTrackerVR Functions Setup
  (`self.Cast Spell By Id` id))

(event `InputAction|SaveGestures`
  (params (Key :type "Key Structure"))
  ;[0.2157 0.4549 1] GestureTrackerVR Functions Setup
  (:`Pressed`
    (`GestureTracker.SaveGestures` (`self.GestureTracker`) (`self.Filename`)) ; Path is relative to your game's content folder
  ))

(event `self.GestureTracker.GestureRecognized`
  (params (id :type Integer) (name :type String) (recognitionDuration :type "Float (single-precision)") (lengthRatio :type "Float (single-precision)"))
  ;[0.2157 0.4549 1] GestureTrackerVR Functions Setup
)

(event `InputAction|ClearGesture`
  (params (Key :type "Key Structure"))
  ;[0.2157 0.4549 1] GestureTrackerVR Functions Setup
  (:`Pressed`
    (`GestureTracker.ClearGestures` (`self.GestureTracker`))))

(event `EnhancedInput|/Game/VRTemplate/Input/Actions/IA_Gesture_Right`
  (params (ActionValue :type Boolean) (ElapsedSeconds :type "Float (double-precision)") (TriggeredSeconds :type "Float (double-precision)") (InputAction :type "InputAction Object Reference" :default "/Game/VRTemplate/Input/Actions/IA_Gesture_Right.IA_Gesture_Right"))
  ;[0.2157 0.4549 1] GestureTrackerVR Functions Setup
  (:`Triggered`
    (goto _label :!via `execute2`))
  (:`Completed`
    (goto _label_2 :!via `execute2`)))

(event `InputAction|ContinuousRight`
  (params (Key :type "Key Structure"))
  (bind _gesturetracker (`self.GestureTracker`))
  ;[0.2157 0.4549 1] GestureTrackerVR Functions Setup
  (:`Pressed`
    (`GestureTracker.StartContinuousRecognition` :`self` _gesturetracker))
  (:`Released`
    (`GestureTracker.StopContinuousRecognition` _gesturetracker)))

(event `InputAction|LoadGestures`
  (params (Key :type "Key Structure"))
  ;[0.2157 0.4549 1] GestureTrackerVR Functions Setup
  (:`Pressed`
    (`GestureTracker.LoadGestures` (`self.GestureTracker`) (`self.Filename`))))

(event `EnhancedInput|/Game/VRTemplate/Input/Actions/IA_Cancel_Left`
  (params (ActionValue :type Boolean) (ElapsedSeconds :type "Float (double-precision)") (TriggeredSeconds :type "Float (double-precision)") (InputAction :type "InputAction Object Reference" :default "/Game/VRTemplate/Input/Actions/IA_Cancel_Left.IA_Cancel_Left"))
  (bind _gesturetracker (`self.GestureTracker`))
  ;[0.2157 0.4549 1] GestureTrackerVR Functions Setup
  (:`Triggered`
    (`self.Get Hand Held` :!label _label_3
      (:`then`
        _)
      (:`then2`
        _))
    (`GestureTracker.StartRecognition` :`self` _gesturetracker))
  (:`Completed`
    (`self.Get Hand Held` :!label _label_4
      (:`then`
        _)
      (:`then2`
        _))
    (bind _id (`GestureTracker.FinishRecognition` _gesturetracker)
      (:`Recognized`
        (bind _output_get (set `self.Id` _id))
        (`self.Cast Spell By Id` _output_get)))))

(event `EnhancedInput|/Game/VRTemplate/Input/Actions/IA_Cancel_Right`
  (params (ActionValue :type Boolean) (ElapsedSeconds :type "Float (double-precision)") (TriggeredSeconds :type "Float (double-precision)") (InputAction :type "InputAction Object Reference" :default "/Game/VRTemplate/Input/Actions/IA_Cancel_Right.IA_Cancel_Right"))
  ;[0.2157 0.4549 1] GestureTrackerVR Functions Setup
  (:`Triggered`
    (goto _label_3 :!via `execute2`))
  (:`Completed`
    (goto _label_4 :!via `execute2`)))

(event `EnhancedInput|/Game/VRTemplate/Input/Actions/IA_Shoot_Left`
  (params (ActionValue :type Boolean) (ElapsedSeconds :type "Float (double-precision)") (TriggeredSeconds :type "Float (double-precision)") (InputAction :type "InputAction Object Reference" :default "/Game/VRTemplate/Input/Actions/IA_Shoot_Left.IA_Shoot_Left"))
  (bind (_currentspellinfo_spellname _currentspellinfo_desciption _currentspellinfo_spelltype _currentspellinfo_spellarea) (break `/Game/Blueprints/Data_Assets/Structs/SpellInfo` (`self.CurrentSpellInfo`)))
  (:`Triggered`
    (`self.Get Hand Held` :!label _label_5
      (:`then`
        _)
      (:`then2`
        _))
    (if (or (`self.SpellForm?`) (== (`self.ElementCount`) 0))
      (`self.FindMatchingSpell` (`self.CurrentSpellInfo`)
        (:`NewParam2`
          (switch `/Game/Blueprints/Data_Assets/enums/SpellAreaType` _currentspellinfo_spellarea
            (:`NewEnumerator0`
              (`self.ProjectileLogic`
                (:`NewParam`
                  _)))
            (:`NewEnumerator1`
              (`self.StreamLogic`
                (:`NewParam`
                  _)))
            (:`NewEnumerator2`
              (`self.AOELogic`
                (:`NewParam`
                  _)))
            (:`NewEnumerator3`
              (`self.TouchLogic`
                (:`NewParam`
                  _))))
          (`self.Reset Variables`)))
      (else
        (`|SpawnActorFromClass` "/Game/Portals_VFXPack/Blueprints/BP_ExampleProjectile.BP_ExampleProjectile_C" (`KismetMathLibrary.MakeTransform` (`SceneComponent.K2_GetComponentLocation` (`self.Sphere`)) (`KismetMathLibrary.Conv_VectorToRotator` (`SceneComponent.GetForwardVector` (`self.Arrow`)))) "Undefined" "OverrideRootScale" null null))))
  (:`Completed`
    (`self.Get Hand Held` :!label _label_6)))

(event `EnhancedInput|/Game/VRTemplate/Input/Actions/IA_Shoot_Right`
  (params (ActionValue :type Boolean) (ElapsedSeconds :type "Float (double-precision)") (TriggeredSeconds :type "Float (double-precision)") (InputAction :type "InputAction Object Reference" :default "/Game/VRTemplate/Input/Actions/IA_Shoot_Right.IA_Shoot_Right"))
  (:`Triggered`
    (goto _label_5 :!via `execute2`))
  (:`Completed`
    (goto _label_6 :!via `execute2`)))

(event `self.Sphere1.OnComponentBeginOverlap`
  (params (OverlappedComponent :type "PrimitiveComponent Object Reference") (OtherActor :type "Actor Object Reference") (OtherComp :type "PrimitiveComponent Object Reference") (OtherBodyIndex :type Integer) (bFromSweep :type Boolean) (SweepResult :type "HitResult Structure (by ref)"))
  (bind _asaot_fb_char (cast `/Game/Blueprints/Character/AOT_FB_Char` OtherActor))
  (set `self.Player` _asaot_fb_char))

(fn `Reset Variables`
  (set `self.Id` 9)
  (set `self.SpellForm?` false)
  (set `self.ElementCount` 0)
  (set `self.Spell Form` "NewEnumerator4")
  (set `self.ElementType` "NewEnumerator4")
  (set `self.CurrentSpellInfo` (struct)))

(fn `UserConstructionScript`)