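; Game mode that keeps a list of connected player controllers and resyncs VR avatar calibration whenever someone joins.
; On post-login it adds the new player, then calls RefreshCalibrationForAllConnectedPlayers on the YnnkVrAvatarComponent of every valid controller in the list that has one.
; On logout it removes the exiting player controller from the list.
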(event `self.K2_PostLogin`
  (params (NewPlayer :type "PlayerController Object Reference"))
  (bind _connectedplayers (`self.ConnectedPlayers`))
  (`KismetArrayLibrary.Array_Add` _connectedplayers NewPlayer)
  (for _array_element _connectedplayers
    (`/Engine/EditorBlueprintResources/StandardMacros.IsValid` _array_element
      (:`Is Valid`
        (bind _returnvalue (`self.GetComponentByClass` _array_element "/Script/VRIKBodyRuntime.YnnkVrAvatarComponent"))
        (`/Engine/EditorBlueprintResources/StandardMacros.IsValid` _returnvalue
          (:`Is Valid`
            (`YnnkVrAvatarComponent.RefreshCalibrationForAllConnectedPlayers` _returnvalue)))))))

(event `self.K2_OnLogout`
  (params (ExitingController :type "Controller Object Reference"))
  (bind _asplayer_controller (cast `PlayerController` ExitingController))
  (`KismetArrayLibrary.Array_RemoveItem` (`self.ConnectedPlayers`) _asplayer_controller))

(fn `UserConstructionScript`)