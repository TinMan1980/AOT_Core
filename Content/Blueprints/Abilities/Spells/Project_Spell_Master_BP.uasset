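; Master spell actor whose appearance and damage come from a SpellDetails struct, so one Blueprint can represent different spells.
; SetSpell applies the struct's mesh, material and two Niagara effects, running on BeginPlay and whenever SetSpellDetails supplies a new struct.
; BeginPlay also repeats those assignments, then switches on spell type with no branch logic attached.
; A hit on the collision sphere applies the struct's base damage to the other actor and destroys the spell.
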(event `self.ReceiveBeginPlay`
  (bind _staticmesh (`self.StaticMesh`))
  (`self.SetSpell`)
  (`StaticMeshComponent.SetStaticMesh` _staticmesh (`self.Spell Details Spell Mesh `))
  (`PrimitiveComponent.SetMaterial` _staticmesh 0 (`self.Spell Details Material `))
  (`NiagaraComponent.SetAsset` (`self.Niagara`) (`self.Spell Details Particle Effect 1 `) true)
  (`NiagaraComponent.SetAsset` (`self.Niagara1`) (`self.Spell Details Particle Effect 2 `) true)
  (switch `/Game/Blueprints/Data_Assets/enums/SpellType` (`self.Spell Details Spell Type`)))

(event `self.Sphere.OnComponentHit`
  (params (HitComponent :type "PrimitiveComponent Object Reference") (OtherActor :type "Actor Object Reference") (OtherComp :type "PrimitiveComponent Object Reference") (NormalImpulse :type "Vector Structure") (Hit :type "HitResult Structure (by ref)"))
  (`GameplayStatics.ApplyDamage` OtherActor (`.BaseDamage_58_57335D9F479B94174D9F12A275D4CC38` (break `/Game/Blueprints/Data_Assets/Structs/SpellInfo` (`self.SpellDetails`))))
  (`self.K2_DestroyActor`))

(fn `Set Spell Details`
  (params (NewParam :type "/Game/Blueprints/Data_Assets/Structs/SpellInfo Structure"))
  (set `self.SpellDetails` NewParam)
  (`self.SetSpell`))

(fn `UserConstructionScript`)